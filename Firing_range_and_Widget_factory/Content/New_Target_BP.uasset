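; New_Target_BP is a shootable target that can slide back and forth and drops when hit.
; If ShouldMove is set, two timelines with a play rate derived from Speed loop it between its starting position and EndLocation.
; Each hit plays an explosion sound; the first chains Falling, Wait and Raising timelines to roll the mesh.
; HasBeenShot blocks retriggering until the target is raised again.
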(event EventBeginPlay
  (Variables|Default|SetHasBeenShot false)
  (if (Variables|Default|GetShould%20move)
    (Variables|Default|SetStartLocation (Transformation|GetActorLocation))
    (Components|Timeline|SetPlayRate (Variables|Default|GetMove%20Left) (/ 1.0 (Variables|Default|GetSpeed)))
    (bind _move_left_track (Timeline|Move%20Left PlayFromStart)
      (:Update
        (Transformation|SetActorRelativeLocation (Math|Vector|Lerp(Vector) (Variables|Default|GetStartLocation) (Variables|Default|GetEnd%20Location) _move_left_track)))
      (:Finished
        (bind _move_right_timeline (Timeline|Move%20Right PlayFromStart)
          (:Update
            (Transformation|SetActorRelativeLocation (Math|Vector|Lerp(Vector) (Variables|Default|GetEnd%20Location) (Variables|Default|GetStartLocation) _move_right_timeline)))
          (:Finished
            (Timeline|Move%20Left PlayFromStart)))))))

(event Collision|EventHit
  (params (MyComp :type Primitive%20Component%20Object%20Reference) (Other :type Actor%20Object%20Reference) (OtherComp :type Primitive%20Component%20Object%20Reference) (bSelfMoved :type Boolean) (HitLocation :type Vector :default "0, 0, 0") (HitNormal :type Vector :default "0, 0, 0") (NormalImpulse :type Vector :default "0, 0, 0") (Hit :type Hit%20Result%20Structure%20%28by%20ref%29))
  (Audio|PlaySoundatLocation "/Game/StarterContent/Audio/Explosion02.Explosion02" (Transformation|GetActorLocation) "0, 0, 0" 1.0 1.0 0.0 0 0 0 0)
  (if (not (Variables|Default|GetHasBeenShot))
    (Variables|Default|SetHasBeenShot true)
    (bind _falling_track (Timeline|Falling PlayFromStart)
      (:Update
        (Transformation|SetRelativeRotation (Variables|Default|GetTarget_mesh) (Math|Rotator|MakeRotator _falling_track 0.0 0.0) false false))
      (:Finished
        (Timeline|Wait PlayFromStart
          (:Finished
            (bind _raising_track (Timeline|Raising PlayFromStart)
              (:Update
                (Transformation|SetRelativeRotation (Variables|Default|GetTarget_mesh) (Math|Rotator|MakeRotator _raising_track 0.0 0.0) false false))
              (:Finished
                (Variables|Default|SetHasBeenShot false)))))))))

(fn ConstructionScript)